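; BP_Paper_Piece is a paper puzzle piece that is moved with the puzzle cursor and locks once placed at its target location.
; BeginPlay enables pickup and rotation and resets its current grid location.
; While picked up, Tick copies X/Y from BP_PuzzleCursor, found with GetActorOfClass.
; When not held and the cursor coordinates match the target, it disables pickup and marks the position correct, ignoring rotation.
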(event `self.ReceiveBeginPlay`
  (`parent.ReceiveBeginPlay`)
  (set `self.DefaultFloor` 123.0)
  (set `self.canPickUp` true)
  (set `self.canRotateLeft` true)
  (set `self.canRotateRight` true)
  (set `self.curLocX` -1)
  (set `self.curLocY` -1))

(event `self.ReceiveTick`
  (params (DeltaSeconds :type "Float (single-precision)"))
  (`parent.ReceiveTick` DeltaSeconds)
  ;[1 1 1] Syncs the Cursor X/Y Loc with the Object X/Y Loc only when the object is picked up.
  (if (`self.isPickedUp`)
    (bind _returnvalue (`GameplayStatics.GetActorOfClass` "/Game/FirstPerson/Blueprints/BP_PuzzleCursor.BP_PuzzleCursor_C"))
    (cast `/Game/FirstPerson/Blueprints/BP_PuzzleCursor` _returnvalue)
    (bind _cursorxloc (`/Game/FirstPerson/Blueprints/BP_PuzzleCursor.cursorXLoc` _returnvalue))
    (set `self.curLocX` _cursorxloc)
    (bind _cursoryloc (`/Game/FirstPerson/Blueprints/BP_PuzzleCursor.cursorYLoc` _returnvalue))
    (set `self.curLocY` _cursoryloc))
  (if (and (== (`self.targetLocX`) _cursorxloc) (== (`self.targetLocY`) _cursoryloc) true)
    (if (not (`self.isPickedUp`))
      (set `self.canPickUp` false)
      (set `self.correctPosition` true))))

(fn `UserConstructionScript`
  (`parent.UserConstructionScript`))