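; BP_Puz_Interact is a puzzle object that can be carried by the puzzle cursor.
; While IsPickedUp is set, Tick looks up the BP_PuzzleCursor actor every frame and follows its location, offset vertically by DistFromCursor.
; A JustPickedUp flag detects release, snapping the object once to the cursor's XY at the DefaultFloor height.
; IsPickedUp is only read here, never set.
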(event `self.ReceiveTick`
  (params (DeltaSeconds :type "Float (single-precision)"))
  (if (`self.isPickedUp`)
    (bind _returnvalue (`GameplayStatics.GetActorOfClass` "/Game/FirstPerson/Blueprints/BP_PuzzleCursor.BP_PuzzleCursor_C"))
    (bind _asbp_puzzle_cursor (cast `/Game/FirstPerson/Blueprints/BP_PuzzleCursor` _returnvalue))
    (bind _returnvalue_2 (`self.K2_GetActorLocation` _asbp_puzzle_cursor))
    (bind (_x _y _z) (`KismetMathLibrary.BreakVector3f` _returnvalue_2))
    (`self.K2_SetActorLocation` (`KismetMathLibrary.MakeVector` _x _y (+ _z (`self.DistFromCursor`))))
    (set `self.JustPickedUp` true)
    (elif (`self.JustPickedUp`)
      (set `self.JustPickedUp` false)
      (bind (_x_2 _y_2) (`KismetMathLibrary.BreakVector3f` _returnvalue_2))
      (`self.K2_SetActorLocation` (`KismetMathLibrary.MakeVector` _x_2 _y_2 (`self.DefaultFloor`))))))

(fn `UserConstructionScript`)