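; BP_PowerEnd is a power endpoint that shows whether an adjacent BP_PowerTile is feeding it power.
; Its Cube's overlap events store the touching actor and an overlap flag.
; Every Tick, CheckPower tests that tile's North, East, South and West colliders against the Cube, looking for a side that is both active and powered.
; The result sets IsPowered and swaps the Cube's material between powered and base looks.
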(event `self.ReceiveTick`
  (params (DeltaSeconds :type "Float (single-precision)"))
  (bind _isrecievingpower (`self.CheckPower`))
  (bind _output_get (set `self.isPowered` _isrecievingpower))
  (if _output_get
    (`PrimitiveComponent.SetMaterial` (`self.Cube`) 0 "/Game/FPWeapon/Materials/FirstPersonProjectileMaterial.FirstPersonProjectileMaterial")
    (else
      (`PrimitiveComponent.SetMaterial` (`self.Cube`) 0 "/Game/FPWeapon/Materials/BaseMaterial.BaseMaterial"))))

(event `self.Cube.OnComponentBeginOverlap`
  (params (OverlappedComponent :type "PrimitiveComponent Object Reference") (OtherActor :type "Actor Object Reference") (OtherComp :type "PrimitiveComponent Object Reference") (OtherBodyIndex :type Integer) (bFromSweep :type Boolean) (SweepResult :type "HitResult Structure (by ref)"))
  (set `self.collidedPlate` OtherActor)
  (set `self.isOverlap` true))

(event `self.Cube.OnComponentEndOverlap`
  (params (OverlappedComponent :type "PrimitiveComponent Object Reference") (OtherActor :type "Actor Object Reference") (OtherComp :type "PrimitiveComponent Object Reference") (OtherBodyIndex :type Integer))
  (set `self.isOverlap` false))

(fn `CheckPower`
  (returns (isRecievingPower :type Boolean))
  (bind _cube (`self.Cube`))
  (if (`self.isOverlap`)
    (bind _asbp_power_tile (cast `/Game/BP_PowerTile` (`self.collidedPlate`)))
    (if (`PrimitiveComponent.IsOverlappingComponent` (`/Game/BP_PowerTile.NorthCollider` _asbp_power_tile) _cube)
      ;[1 1 1] North Detection
      (if (`/Game/BP_PowerTile.NorthActive` _asbp_power_tile)
        (if (`/Game/BP_PowerTile.NorthPower` _asbp_power_tile)
          (return true)
          (else
            (if (`PrimitiveComponent.IsOverlappingComponent` (`/Game/BP_PowerTile.EastCollider` _asbp_power_tile) _cube) :!label _label
              ;[1 1 1] East Detection
              (if (`/Game/BP_PowerTile.EastActive` _asbp_power_tile)
                (if (`/Game/BP_PowerTile.EastPower` _asbp_power_tile)
                  (return true)
                  (else
                    (if (`PrimitiveComponent.IsOverlappingComponent` (`/Game/BP_PowerTile.SouthCollider` _asbp_power_tile) _cube) :!label _label_2
                      ;[1 1 1] South Detection
                      (if (`/Game/BP_PowerTile.SouthActive` _asbp_power_tile)
                        (if (`/Game/BP_PowerTile.SouthPower` _asbp_power_tile)
                          (return true)
                          (else
                            (if (`PrimitiveComponent.IsOverlappingComponent` (`/Game/BP_PowerTile.WestCollider` _asbp_power_tile) _cube) :!label _label_3
                              ;[1 1 1] West Detection
                              (if (`/Game/BP_PowerTile.WestActive` _asbp_power_tile)
                                (if (`/Game/BP_PowerTile.WestPower` _asbp_power_tile)
                                  (return true)
                                  (else
                                    _)))
                              (return false))))
                        (else
                          (goto _label_3)))
                      (else
                        (goto _label_3)))))
                (else
                  (goto _label_2)))
              (else
                (goto _label_2)))))
        (else
          (goto _label)))
      (else
        (goto _label)))
    (else
      (return false))))

(fn `UserConstructionScript`)