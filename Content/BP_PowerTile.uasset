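; BP_PowerTile is a wire tile that carries power from a BP_Powersource through neighboring tiles.
; Four side colliders track overlaps, and Tick polls each active side through CheckPower for a source or matching powered wire.
; PowerLevel counts hops from the source, accepting only neighbors one level lower so tiles avoid powering each other in loops.
; Powered state spreads to active sides, and wire materials show powered, unpowered or inactive.
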(event `self.ReceiveBeginPlay`
  (`parent.ReceiveBeginPlay`)
  (set `self.canPickUp` true)
  (set `self.canRotateLeft` true)
  (set `self.canRotateRight` true)
  (set `self.DistFromCursor` -160.0)
  (set `self.DefaultFloor` 40.0))

(event `self.ReceiveTick`
  (params (DeltaSeconds :type "Float (single-precision)"))
  (`parent.ReceiveTick` DeltaSeconds)
  (`self.InternalPowerCode`)
  (`self.VisualPowerCode`)
  (bind _isrecievingpower (`self.CheckPower` (`self.NorthActive`) (`self.isNorthOverlap`) (`self.NorthOverlap`) (`self.NorthCollider`))) ; Checking Is North
  (bind _isrecievingpower_2 (`self.CheckPower` (`self.EastActive`) (`self.isEastOverlap`) (`self.EastOverlap`) (`self.EastCollider`))) ; Checking Is East
  (bind _isrecievingpower_3 (`self.CheckPower` (`self.SouthActive`) (`self.isSouthOverlap`) (`self.SouthOverlap`) (`self.SouthCollider`))) ; Checking Is South
  (bind _isrecievingpower_4 (`self.CheckPower` (`self.WestActive`) (`self.isWestOverlap`) (`self.WestOverlap`) (`self.WestCollider`))) ; Checking Is West
  (if (or _isrecievingpower _isrecievingpower_2 _isrecievingpower_3 _isrecievingpower_4)
    (set `self.isPowered` true)
    (else
      (set `self.isPowered` false)
      (set `self.powerLevel` 0))))

(event `self.EastCollider.OnComponentBeginOverlap`
  (params (OverlappedComponent :type "PrimitiveComponent Object Reference") (OtherActor :type "Actor Object Reference") (OtherComp :type "PrimitiveComponent Object Reference") (OtherBodyIndex :type Integer) (bFromSweep :type Boolean) (SweepResult :type "HitResult Structure (by ref)"))
  ;[1 1 1] Detecting if there is overlap
  (set `self.EastOverlap` OtherActor)
  (set `self.isEastOverlap` true))

(event `self.SouthCollider.OnComponentBeginOverlap`
  (params (OverlappedComponent :type "PrimitiveComponent Object Reference") (OtherActor :type "Actor Object Reference") (OtherComp :type "PrimitiveComponent Object Reference") (OtherBodyIndex :type Integer) (bFromSweep :type Boolean) (SweepResult :type "HitResult Structure (by ref)"))
  ;[1 1 1] Detecting if there is overlap
  (set `self.SouthOverlap` OtherActor)
  (set `self.isSouthOverlap` true))

(event `self.WestCollider.OnComponentBeginOverlap`
  (params (OverlappedComponent :type "PrimitiveComponent Object Reference") (OtherActor :type "Actor Object Reference") (OtherComp :type "PrimitiveComponent Object Reference") (OtherBodyIndex :type Integer) (bFromSweep :type Boolean) (SweepResult :type "HitResult Structure (by ref)"))
  ;[1 1 1] Detecting if there is overlap
  (set `self.WestOverlap` OtherActor)
  (set `self.isWestOverlap` true))

(event `self.NorthCollider.OnComponentBeginOverlap`
  (params (OverlappedComponent :type "PrimitiveComponent Object Reference") (OtherActor :type "Actor Object Reference") (OtherComp :type "PrimitiveComponent Object Reference") (OtherBodyIndex :type Integer) (bFromSweep :type Boolean) (SweepResult :type "HitResult Structure (by ref)"))
  ;[1 1 1] Detecting if there is overlap
  (set `self.NorthOverlap` OtherActor)
  (set `self.isNorthOverlap` true))

(event `self.SouthCollider.OnComponentEndOverlap`
  (params (OverlappedComponent :type "PrimitiveComponent Object Reference") (OtherActor :type "Actor Object Reference") (OtherComp :type "PrimitiveComponent Object Reference") (OtherBodyIndex :type Integer))
  ;[1 1 1] Detecting if there is overlap
  (set `self.isSouthOverlap` false))

(event `self.WestCollider.OnComponentEndOverlap`
  (params (OverlappedComponent :type "PrimitiveComponent Object Reference") (OtherActor :type "Actor Object Reference") (OtherComp :type "PrimitiveComponent Object Reference") (OtherBodyIndex :type Integer))
  ;[1 1 1] Detecting if there is overlap
  (set `self.isWestOverlap` false))

(event `self.EastCollider.OnComponentEndOverlap`
  (params (OverlappedComponent :type "PrimitiveComponent Object Reference") (OtherActor :type "Actor Object Reference") (OtherComp :type "PrimitiveComponent Object Reference") (OtherBodyIndex :type Integer))
  ;[1 1 1] Detecting if there is overlap
  (set `self.isEastOverlap` false))

(event `self.NorthCollider.OnComponentEndOverlap`
  (params (OverlappedComponent :type "PrimitiveComponent Object Reference") (OtherActor :type "Actor Object Reference") (OtherComp :type "PrimitiveComponent Object Reference") (OtherBodyIndex :type Integer))
  ;[1 1 1] Detecting if there is overlap
  (set `self.isNorthOverlap` false))

(fn `CheckPower`
  (params (DirActive :type Boolean) (isDirOverlap :type Boolean) (dirOverlap :type "Object Object Reference") (dirCollider :type "BoxComponent Object Reference"))
  (returns (isRecievingPower :type Boolean))
  (bind _powerlevel (`self.powerLevel`))
  (if DirActive
    (if isDirOverlap
      (bind _asbp_power_tile (cast `/Game/BP_PowerTile` dirOverlap)
        (:`then`
          (if (`/Game/BP_PowerTile.isPowered` _asbp_power_tile)
            (if (`PrimitiveComponent.IsOverlappingComponent` (`/Game/BP_PowerTile.NorthCollider` _asbp_power_tile) dirCollider)
              ;[1 1 1] North Detection
              (if (`/Game/BP_PowerTile.NorthActive` _asbp_power_tile)
                (if (`/Game/BP_PowerTile.NorthPower` _asbp_power_tile)
                  (if (== _powerlevel 0) :!label _label
                    (bind _returnvalue (+ (`/Game/BP_PowerTile.powerLevel` _asbp_power_tile) 1))
                    (set `self.powerLevel` _returnvalue))
                  (if (== _powerlevel _returnvalue)
                    (return true)
                    (else
                      (return false)))
                  (else
                    (if (`PrimitiveComponent.IsOverlappingComponent` (`/Game/BP_PowerTile.EastCollider` _asbp_power_tile) dirCollider) :!label _label_2
                      ;[1 1 1] East Detection
                      (if (`/Game/BP_PowerTile.EastActive` _asbp_power_tile)
                        (if (`/Game/BP_PowerTile.EastPower` _asbp_power_tile)
                          (goto _label)
                          (else
                            _))))
                    (if (`PrimitiveComponent.IsOverlappingComponent` (`/Game/BP_PowerTile.SouthCollider` _asbp_power_tile) dirCollider)
                      ;[1 1 1] South Detection
                      (if (`/Game/BP_PowerTile.SouthActive` _asbp_power_tile)
                        (if (`/Game/BP_PowerTile.SouthPower` _asbp_power_tile)
                          (goto _label)
                          (else
                            _))))
                    (bind _westcollider (`/Game/BP_PowerTile.WestCollider` _asbp_power_tile))
                    (if (`PrimitiveComponent.IsOverlappingComponent` _westcollider dirCollider)
                      ;[1 1 1] West Detection
                      (if (`/Game/BP_PowerTile.WestActive` _asbp_power_tile)
                        (if (`/Game/BP_PowerTile.WestPower` _asbp_power_tile)
                          (goto _label)
                          (else
                            _)))
                      (return false)
                      (else
                        _))))
                (else
                  (goto _label_2)))
              (else
                (goto _label_2)))
            (`KismetSystemLibrary.PrintString` (`KismetSystemLibrary.GetDisplayName` _westcollider))
            (else
              (return false))))
        (:`CastFailed`
          (bind _asbp_powersource (cast `/Game/BP_Powersource` dirOverlap)
            (:`then`
              (if (`PrimitiveComponent.IsOverlappingActor` dirCollider _asbp_powersource)
                (set `self.powerLevel` 1)
                (return true)))
            (:`CastFailed`
              (`KismetSystemLibrary.PrintString` "Hello")))))
      (else
        (return false)))))

(fn `InternalPowerCode`
  ;[1 1 1] Power Everything Else
  (if (`self.isPowered`)
    (if (`self.NorthActive`)
      (set `self.NorthPower` true)
      (else
        (set `self.NorthPower` false)))
    (if (`self.EastActive`)
      (set `self.EastPower` true)
      (else
        (set `self.EastPower` false)))
    (if (`self.SouthActive`)
      (set `self.SouthPower` true)
      (else
        (set `self.SouthPower` false)))
    (if (`self.WestActive`)
      (set `self.WestPower` true)
      (else
        (set `self.WestPower` false)))
    (else
      (set `self.NorthPower` false)
      (set `self.EastPower` false)
      (set `self.SouthPower` false)
      (set `self.WestPower` false))))

(fn `UserConstructionScript`
  (`parent.UserConstructionScript`))

(fn `VisualPowerCode`
  (bind _middlewire (`self.MiddleWire`))
  (bind _eastwire (`self.EastWire`))
  (bind _southwire (`self.SouthWire`))
  (bind _northwire (`self.NorthWire`))
  (bind _westwire (`self.WestWire`))
  (if (`self.NorthActive`)
    (if (`self.NorthPower`)
      (`PrimitiveComponent.SetMaterial` _northwire 0 "/Game/FPWeapon/Materials/FirstPersonProjectileMaterial.FirstPersonProjectileMaterial")
      (else
        (`PrimitiveComponent.SetMaterial` _northwire 0 "/Game/FPWeapon/Materials/BaseMaterial.BaseMaterial")))
    (else
      (`PrimitiveComponent.SetMaterial` _northwire 0 "/Game/StarterContent/Materials/M_Glass.M_Glass")))
  (if (`self.EastActive`)
    (if (`self.EastPower`)
      (`PrimitiveComponent.SetMaterial` _eastwire 0 "/Game/FPWeapon/Materials/FirstPersonProjectileMaterial.FirstPersonProjectileMaterial")
      (else
        (`PrimitiveComponent.SetMaterial` _eastwire 0 "/Game/FPWeapon/Materials/BaseMaterial.BaseMaterial")))
    (else
      (`PrimitiveComponent.SetMaterial` _eastwire 0 "/Game/StarterContent/Materials/M_Glass.M_Glass")))
  (if (`self.SouthActive`)
    (if (`self.SouthPower`)
      (`PrimitiveComponent.SetMaterial` _southwire 0 "/Game/FPWeapon/Materials/FirstPersonProjectileMaterial.FirstPersonProjectileMaterial")
      (else
        (`PrimitiveComponent.SetMaterial` _southwire 0 "/Game/FPWeapon/Materials/BaseMaterial.BaseMaterial")))
    (else
      (`PrimitiveComponent.SetMaterial` _southwire 0 "/Game/StarterContent/Materials/M_Glass.M_Glass")))
  (if (`self.WestActive`)
    (if (`self.WestPower`)
      (`PrimitiveComponent.SetMaterial` _westwire 0 "/Game/FPWeapon/Materials/FirstPersonProjectileMaterial.FirstPersonProjectileMaterial")
      (else
        (`PrimitiveComponent.SetMaterial` _westwire 0 "/Game/FPWeapon/Materials/BaseMaterial.BaseMaterial")))
    (else
      (`PrimitiveComponent.SetMaterial` _westwire 0 "/Game/StarterContent/Materials/M_Glass.M_Glass")))
  (if (`self.isPowered`)
    (`PrimitiveComponent.SetMaterial` _middlewire 0 "/Game/FPWeapon/Materials/FirstPersonProjectileMaterial.FirstPersonProjectileMaterial")
    (else
      (`PrimitiveComponent.SetMaterial` _middlewire 0 "/Game/FPWeapon/Materials/BaseMaterial.BaseMaterial"))))