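; Player inventory component that stores item stacks, creates the HUD and handles interact, hotbar-scroll and menu keys.
; A camera sphere trace each tick picks the looked-at actor, which E interacts with if it has item data.
; Adding fills stacks one unit at a time up to data-table limits, then empty slots, returning any remainder.
; Tick also resizes slots to track filled count plus one, minimum three; removal is an empty stub.
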(event `self.ReceiveTick`
  (params (DeltaSeconds :type "Float (single-precision)"))
  (`self.Interaction Trace`)
  (`self.Resize Inventory`) ; Sets the default array size
  ;[1 1 1] Checks how many items are in inventory
  (set `self.TotalItems` 0)
  (for _array_element (`self.Content`)
    (if (not (== (`.ItemID_2_0442506E473F88A76E417D83CBC4EA2C` (break `/Game/Inventory_System/FSlotStruct` _array_element)) "None"))
      (`/Engine/EditorBlueprintResources/StandardMacros.IncrementInt` (`self.TotalItems`))))
  ;[1 1 1] Sets the inventory size
  (set `self.Inventory Size` (+ (`self.TotalItems`) 1)))

(event `self.ReceiveBeginPlay`
  ;[1 1 1] Sets the size of the inventory array
  (`self.Resize Inventory`) ; Sets the default array size
  ;[1 1 1] Makes the Player HUD widget
  (bind _returnvalue (`|CreateWidget` "/Game/Inventory_System/UI/BPW_PlayerHUD.BPW_PlayerHUD_C"))
  (bind _output_get (set `self.HUD` _returnvalue))
  (`UserWidget.AddToViewport` _output_get 0))

(event `Key|E`
  (params (Key :type "Key Structure"))
  (:`Pressed`
    (bind _look_at_actor (`self.Look at Actor`) ; Checks if the Look at Actor Var is empty or not
      (:`then`
        (bind _returnvalue (`Actor.GetComponentByClass` _look_at_actor "/Game/Inventory_System/BPC_ItemData.BPC_ItemData_C"))
        ;[1 1 1] Checks to see if object is an item
        (`/Engine/EditorBlueprintResources/StandardMacros.IsValid` _returnvalue
          (:`Is Valid`
            ;[1 1 1] Calls the "Interact With" Interface
            (message `/Game/Inventory_System/BPI_InteractInterface.InteractWith` _returnvalue (cast `/Game/FirstPerson/Blueprints/testcharacter` (`self.GetOwner`) :!pure true))
            (`self.MC_Update`))))
      (:`else`))))

(event `Key|One`
  (params (Key :type "Key Structure"))
  (:`Pressed`
    (`self.DEBUG_PRINTCONTENTS`)))

(event `Key|R`
  (params (Key :type "Key Structure"))
  ;[1 1 1] Hotbar Scroll Controls
  (:`Pressed`
    (bind _result (`/Engine/EditorBlueprintResources/StandardMacros.DecrementInt` (`self.HotbarIndex`))
      (:`  `
        ;[1 1 1] Bottom bracket for Hotbar Index
        (if (< _result 0)
          (set `self.HotbarIndex` (- (`self.Inventory Size`) 1)) ; Set HotbarIndex to Inventory Size
        )
        (`self.MC_Update` :!label _label)))))

(event `Key|T`
  (params (Key :type "Key Structure"))
  ;[1 1 1] Hotbar Scroll Controls
  (:`Pressed`
    (bind _result (`/Engine/EditorBlueprintResources/StandardMacros.IncrementInt` (`self.HotbarIndex`))
      (:`  `
        ;[1 1 1] Top Bracket for Hotbar Index
        (if (> _result (- (`self.Inventory Size`) 1))
          (set `self.HotbarIndex` 0) ; Set Hotbar Index to 0
          (goto _label)
          (else
            (goto _label)))))))

(event `Key|Two`
  (params (Key :type "Key Structure"))
  ;[1 1 1] Show Inventory
  (:`Pressed`
    (`/Game/Inventory_System/UI/BPW_PlayerHUD.DisplayPlayerMenu` (`self.HUD`))))

(event `MC_Update`
  (`self.OnInventoryUpdated`))

(fn `Add Item to Inventory`
  (params (ItemID :type "Name (by ref)") (Quantity :type Integer))
  (returns (Success :type Boolean) (`Quantity Remaining` :type Integer))
  (locals (Local_QuantityRemaining :type Integer) (Local_HasFailed :type Boolean))
  (bind _output_get (set `local.Local_QuantityRemaining` Quantity)) ; This only runs once
  (while (and (> (`local.Local_QuantityRemaining`) 0) (not (`local.Local_HasFailed`)))
    (bind (_index _found_slot) (`self.Find Slot` ItemID)) ; Checks to see if a slot exists for the item
    (if _found_slot
      ;[1 1 1] Adds !!!1!!! item to stack then removes from quantity
      (`self.Add to Stack` _index 1)
      (`/Engine/EditorBlueprintResources/StandardMacros.DecrementInt` (`local.Local_QuantityRemaining`))
      (elif (`self.Any Empty Slots Available`)
        ;[1 1 1] Creates a new Stack Then removes 1 from the total quantity
        (bind _success (`self.Create New Stack` (`local.ItemID`) 1)) ; Creates a new stack with value of !!!1!!!
        (if _success
          (`/Engine/EditorBlueprintResources/StandardMacros.DecrementInt` (`local.Local_QuantityRemaining`))
          (else
            (set `local.Local_HasFailed` true)))
        (else
          (set `local.Local_HasFailed` true)))))
  (return (not (`local.Local_HasFailed`)) _output_get))

(fn `Add to Stack`
  (params (Index :type Integer) (Quantity :type Integer))
  (bind (_output_itemid _output_quantity) (break `/Game/Inventory_System/FSlotStruct` (`|GetArrayItem` (`self.Content`) Index)))
  (`KismetArrayLibrary.Array_Set` (`self.Content`) Index (make `/Game/Inventory_System/FSlotStruct` _output_itemid (+ Quantity _output_quantity))))

(fn `Any Empty Slots Available`
  (returns (HasEmptySlot :type Boolean) (EmptyIndex :type Integer))
  (for (_array_element _array_index) (`self.Content`)
    (if (== (`.Quantity_5_B78DCF314DECD01A5B65829375D89854` (break `/Game/Inventory_System/FSlotStruct` _array_element)) 0)
      (return true _array_index) ; EmptyIndex = The slot that's empty
    ))
  (return false -1) ; If No EMpty Slots :(((
)

(fn `Create New Stack`
  (params (ItemID :type Name) (Quantity :type Integer))
  (returns (Success :type Boolean))
  (bind (_hasemptyslot _emptyindex) (`self.Any Empty Slots Available`))
  (if _hasemptyslot
    (`KismetArrayLibrary.Array_Set` (`self.Content`) _emptyindex (make `/Game/Inventory_System/FSlotStruct` ItemID Quantity))
    (return true)
    (else
      (return false))))

(fn `DEBUG_PRINTCONTENTS`
  (for (_array_element _array_index) (`self.Content`)
    (bind (_itemid _quantity) (break `/Game/Inventory_System/FSlotStruct` _array_element))
    (`KismetSystemLibrary.PrintString` (`KismetStringLibrary.Concat_StrStr` (`KismetStringLibrary.Conv_IntToString` _array_index) ": " (`KismetStringLibrary.Conv_NameToString` _itemid) " = " (`KismetStringLibrary.Conv_IntToString` _quantity)))))

(fn `Find Slot`
  (params (ItemID :type Name))
  (returns (Index :type Integer) (`Found Slot` :type Boolean))
  (for (_array_element _array_index) (`self.Content`)
    (bind (_itemid _quantity) (break `/Game/Inventory_System/FSlotStruct` _array_element))
    (if (== _itemid ItemID)
      (if (< _quantity (`self.Get Max Stack Size` ItemID))
        (return _array_index true))))
  (return -1 false) ; Fail State IFNO SLOT IS FOUND
)

(fn `Get Max Stack Size`
  (params (ItemID :type Name))
  (returns (StackSize :type Integer))
  (bind _returnvalue (`|GetDataTableRow` "/Game/Inventory_System/ItemData.ItemData" ItemID)
    (:`then`
      ;[1 1 1] Gets the max stack size and returns it
      (return (`.StackSize_17_C6ED12214E976D5941B0E18FFF58A03F` (break `/Game/Inventory_System/FItemStruct` _returnvalue))))
    (:`RowNotFound`
      (`KismetSystemLibrary.PrintString` "you fucked up and an item ID is wrong."))))

(fn `Interaction Trace`
  (bind _returnvalue (`GameplayStatics.GetPlayerCameraManager` 0))
  (bind _returnvalue_2 (`Actor.K2_GetActorLocation` _returnvalue))
  (bind (_outhit _returnvalue_3) (`KismetSystemLibrary.SphereTraceSingle` _returnvalue_2 (+ _returnvalue_2 (* (`Actor.GetActorForwardVector` _returnvalue) (`self.Interact Distance`))) 15.0 "TraceTypeQuery3" false (`|MakeArray` (`self.GetOwner`))))
  (if _returnvalue_3
    (bind (_bblockinghit _binitialoverlap _time _distance _location _impactpoint _normal _impactnormal _physmat _hitactor) (`GameplayStatics.BreakHitResult` _outhit))
    ;[1 1 1] This makes it so it doesn't run the same code twice for the same actor
    (if (!= _hitactor (`self.Look at Actor`))
      (bind _output_get (set `self.Look at Actor` _hitactor))
      (bind _message (message `/Game/Inventory_System/BPI_InteractInterface.LookAt` _output_get))
      (`KismetSystemLibrary.PrintText` _message))
    (else
      (set `self.Look at Actor` null) ; Reset's the lookat actor
    )))

(fn `Remove From Inventory`)

(fn `Resize Inventory`
  (if (< (`self.Inventory Size`) 3)
    ;[1 1 1] Inventory Array Size == 3
    (`KismetArrayLibrary.Array_Resize` (`self.Content`) 3)
    (else
      ;[1 1 1] Inventory Array Size = Total Items + 1
      (`KismetArrayLibrary.Array_Resize` (`self.Content`) (`self.Inventory Size`)))))