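; BP_Item is a world item actor for the inventory system that supplies a pickup prompt and can remove itself.
; LookAt reads the item's data table row through the ID on its item data component and returns "Pick up {item}" with the row's name.
; Destroy_Item destroys the actor after a brief delay.
; PickUpItem is empty, with its print, destroy and return-item nodes left disconnected.
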(event `Destroy_Item`
  (`KismetSystemLibrary.Delay` 0.1)
  (`self.K2_DestroyActor`))

(fn `LookAt`
  (returns (Message :type Text))
  (bind (_itemid_datatable _itemid_rowname) (break `DataTableRowHandle` (`/Game/Inventory_System/BPC_ItemData.ItemID` (`self.BPC_ItemData`))))
  ;[1 1 1] Getting data of the item being looked at
  (bind _returnvalue (`|GetDataTableRow` _itemid_datatable _itemid_rowname)
    (:`then`
      (return (`|FormatText` "Pick up {item}" (`.Name_6_DC0A87F248AB13CCC1642D9B39A444F9` (break `/Game/Inventory_System/FItemStruct` _returnvalue)))))))

(fn `Pick Up Item`
  (returns (item :type String)))

(fn `UserConstructionScript`)